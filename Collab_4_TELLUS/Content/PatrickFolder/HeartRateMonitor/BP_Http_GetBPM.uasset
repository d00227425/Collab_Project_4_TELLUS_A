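; Heart rate monitor Blueprint that turns a BPM reading fetched over HTTP into paced astronaut breathing audio.
; Tick passes through a 15-second Delay to send a GET request, then parses and prints the JSON "last_value" field as BPM.
; A looping Delay chain alternates 2D inhale and exhale sounds at intervals inversely proportional to BPM.
; The request URL is empty in this graph.
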(event `self.ReceiveTick`
  (params (DeltaSeconds :type "Float (single-precision)"))
  (bind _returnvalue (/ 1.0 (/ (`self.BPM`) 100.0)))
  (`KismetSystemLibrary.Delay` 15.0)
  (bind (_outheader _result_body) (`|HttpRequest` "" "Get")
    (:`On Success`
      (bind _outjsonobject (`JsonBlueprintFunctionLibrary.FromString` _result_body))
      (bind _outvalue (`|GetJsonField` _outjsonobject "last_value"))
      (`KismetSystemLibrary.PrintString` (`KismetStringLibrary.Conv_IntToString` _outvalue) true true (struct :`G` 0.66 :`B` 1.0 :`A` 1.0) 4.0)
      (set `self.BPM` (`KismetMathLibrary.Conv_IntToDouble` _outvalue))
      ;[1 1 1] Takes heartrate and simulates the pace of breathing in comparison to one's heartrate
      (`KismetSystemLibrary.Delay` _returnvalue :!label _label)
      (`GameplayStatics.PlaySound2D` "/Game/PatrickFolder/HeartRateMonitor/AstronautInhale.AstronautInhale" 1.0 1.0 0.0 null null)
      (`KismetSystemLibrary.Delay` _returnvalue)
      (`GameplayStatics.PlaySound2D` "/Game/PatrickFolder/HeartRateMonitor/AstronautExhale.AstronautExhale" 1.0 1.0 0.0 null null)
      (goto _label))))

(fn `UserConstructionScript`)