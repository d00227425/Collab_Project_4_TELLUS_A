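; VR airlock-style double door that drives a real-world fan through Adafruit IO.
; End triggers open their door via timelines and record the VR pawn's entry side, both checking only door A's lock.
; The middle trigger closes and locks both doors, updates red/green lock materials, spawns a Niagara effect and POSTs fan "on".
; On success it waits, unlocks, POSTs "off", then opens the opposite door once that request succeeds.
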(event `self.ReceiveBeginPlay`
  ;[1 1 1] Set Locks On Spawn
  (`|ExecutionSequence`
    (:`then_0`
      (if (`self.DoorBLocked`)
        (`self.LockDoorB`)
        (else
          (`self.UnlockDoorB`))))
    (:`then_1`
      (if (`self.DoorALocked`)
        (`self.LockDoorA`)
        (else
          (`self.UnlockDoorA`))))))

(event `self.BegingingCollision.OnComponentBeginOverlap`
  (params (OverlappedComponent :type "PrimitiveComponent Object Reference") (OtherActor :type "Actor Object Reference") (OtherComp :type "PrimitiveComponent Object Reference") (OtherBodyIndex :type Integer) (bFromSweep :type Boolean) (SweepResult :type "HitResult Structure (by ref)"))
  (cast `/Game/VRTemplate/Blueprints/VRPawn` OtherActor)
  (if (not (`self.DoorALocked`))
    (set `self.FrontSide` false)
    (bind (_direction _door_a_move) (`Timeline|Door-A-Move` :!label _label)
      (:`Update`
        (`SceneComponent.K2_SetRelativeLocationAndRotation` :`self` (`self.Door1A`) :`NewLocation` (`KismetMathLibrary.MakeVector` 0.0 0.0 _door_a_move))))))

(event `self.BegingingCollision.OnComponentEndOverlap`
  (params (OverlappedComponent :type "PrimitiveComponent Object Reference") (OtherActor :type "Actor Object Reference") (OtherComp :type "PrimitiveComponent Object Reference") (OtherBodyIndex :type Integer))
  (cast `/Game/VRTemplate/Blueprints/VRPawn` OtherActor)
  (if (not (`self.DoorALocked`))
    (goto _label :!via `Reverse`)))

(event `self.MiddleCollision.OnComponentBeginOverlap`
  (params (OverlappedComponent :type "PrimitiveComponent Object Reference") (OtherActor :type "Actor Object Reference") (OtherComp :type "PrimitiveComponent Object Reference") (OtherBodyIndex :type Integer) (bFromSweep :type Boolean) (SweepResult :type "HitResult Structure (by ref)"))
  (cast `/Game/VRTemplate/Blueprints/VRPawn` OtherActor)
  (`|ExecutionSequence`
    (:`then_0`
      (goto _label :!via `Reverse`))
    (:`then_1`
      (bind (_direction _door_a_move) (`Timeline|Timeline` :!via `Reverse` :!label _label_2)
        (:`Update`
          (`SceneComponent.K2_SetRelativeLocationAndRotation` :`self` (`self.Door2A`) :`NewLocation` (`KismetMathLibrary.MakeVector` 0.0 505.0 _door_a_move)))))
    (:`then_2`
      (`self.LockDoorA`)
      (`self.LockDoorB`)
      (`KismetSystemLibrary.Delay` 1.5)
      (`AddComponent|NODE_AddNiagaraComponent-0` :`RelativeTransform` (`KismetMathLibrary.MakeTransform` (0.0 250.0 -50.0) (struct) (3.0 3.0 3.0)))
      (bind _output_get (set `self.StringBody` "{\"x-aio-key\":\"\", \"value\":\"on\"}"))
      (bind (_outheader _result_body) (`|HttpRequest` "https://io.adafruit.com/api/v2/OdhranW/feeds/fan-feed/data" "Post" (struct) _output_get)
        (:`On Success`
          (`KismetSystemLibrary.PrintString` _result_body true true (struct :`G` 0.66 :`B` 1.0 :`A` 1.0) 5.0)
          (`KismetSystemLibrary.Delay` 1.5)
          (`self.UnlockDoorA`)
          (`self.UnlockDoorB`)
          (bind _output_get_2 (set `self.StringBody` "{\"x-aio-key\":\"\", \"value\":\"off\"}"))
          (bind (_outheader_2 _result_body_2) (`|HttpRequest` "https://io.adafruit.com/api/v2/OdhranW/feeds/fan-feed/data" "Post" (struct) _output_get_2)
            (:`On Success`
              (`KismetSystemLibrary.PrintString` _result_body_2 true true (struct :`G` 0.66 :`B` 1.0 :`A` 1.0) 5.0)
              (if (`self.FrontSide`)
                (goto _label)
                (else
                  (goto _label_2))))))))))

(event `self.EndCollision.OnComponentBeginOverlap`
  (params (OverlappedComponent :type "PrimitiveComponent Object Reference") (OtherActor :type "Actor Object Reference") (OtherComp :type "PrimitiveComponent Object Reference") (OtherBodyIndex :type Integer) (bFromSweep :type Boolean) (SweepResult :type "HitResult Structure (by ref)"))
  (cast `/Game/VRTemplate/Blueprints/VRPawn` OtherActor)
  (if (not (`self.DoorALocked`))
    (set `self.FrontSide` true)
    (goto _label_2)))

(event `self.EndCollision.OnComponentEndOverlap`
  (params (OverlappedComponent :type "PrimitiveComponent Object Reference") (OtherActor :type "Actor Object Reference") (OtherComp :type "PrimitiveComponent Object Reference") (OtherBodyIndex :type Integer))
  (cast `/Game/VRTemplate/Blueprints/VRPawn` OtherActor)
  (if (not (`self.DoorALocked`))
    (goto _label_2 :!via `Reverse`)))

(fn `LockDoorA`
  (set `self.DoorALocked` true)
  (`PrimitiveComponent.SetMaterial` (`self.LockA`) 0 "/Game/Odhran_Folder/Quick_Materials/Red.Red"))

(fn `LockDoorB`
  (set `self.DoorBLocked` true)
  (`PrimitiveComponent.SetMaterial` (`self.LockB`) 0 "/Game/Odhran_Folder/Quick_Materials/Red.Red"))

(fn `UnlockDoorA`
  (set `self.DoorALocked` false)
  (`PrimitiveComponent.SetMaterial` (`self.LockA`) 0 "/Game/Odhran_Folder/Quick_Materials/Green.Green"))

(fn `UnlockDoorB`
  (set `self.DoorBLocked` false)
  (`PrimitiveComponent.SetMaterial` (`self.LockB`) 0 "/Game/Odhran_Folder/Quick_Materials/Green.Green"))

(fn `UserConstructionScript`)